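; Physics-driven walking player pawn that moves by lifting and swinging two constrained legs with impulses, plus an axis that pushes the body.
; Timelines raise each leg's constraint target and limit, tinting the lifted leg red.
; On PC, mouse buttons select legs; otherwise one Move axis drives the active leg, alternating on release if a body-to-leg angle check passes.
; Sphere overlap respawns and repossesses a fresh pawn at PlayerStart.
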(event OnComponentBeginOverlap(Sphere)
  (params (OverlappedComponent :type Primitive%20Component%20Object%20Reference) (OtherActor :type Actor%20Object%20Reference) (OtherComp :type Primitive%20Component%20Object%20Reference) (OtherBodyIndex :type Integer) (bFromSweep :type Boolean) (SweepResult :type Hit%20Result%20Structure%20%28by%20ref%29))
  (CallFunction|Spawn))

(event Custom|LiftRight
  (params (isLift :type Boolean))
  (bind _physicsconstraintright (Variables|Default|GetPhysicsConstraintRight))
  (Rendering|Material|SetVectorParameterValue (Variables|Default|GetRightMaterialInstance) "Color" (Math|Color|SelectColor "(R=1.000000,G=0.000000,B=0.000000,A=1.000000)" "(R=1.000000,G=1.000000,B=1.000000,A=1.000000)" isLift) :!class /Script/Engine.MaterialInstanceDynamic)
  (if isLift
    (bind _新建轨道_0 (Timeline|timeline_Right Play)
      (:Update
        (Class|PhysicsConstraintComponent|SetLinearZLimit _physicsconstraintright "LCM_Limited" (Math|Float|Lerp 0.0 (Variables|Default|GetLimit%20Size) _新建轨道_0))
        (Class|PhysicsConstraintComponent|SetLinearPositionTarget _physicsconstraintright (Math|Vector|MakeVector 0.0 0.0 (Math|Float|Lerp 0.0 (Variables|Default|GetLimit%20Size) _新建轨道_0)))))
    (else
      (Timeline|timeline_Right Reverse))))

(event Custom|LIftLeft
  (params (isLift :type Boolean))
  (bind _physicsconstraintleft (Variables|Default|GetPhysicsConstraintLeft))
  (Rendering|Material|SetVectorParameterValue (Variables|Default|Get%20LeftMaterialInstance) "Color" (Math|Color|SelectColor "(R=1.000000,G=0.000000,B=0.000000,A=1.000000)" "(R=1.000000,G=1.000000,B=1.000000,A=1.000000)" isLift) :!class /Script/Engine.MaterialInstanceDynamic)
  (if isLift
    (bind _新建轨道_0 (Timeline|timeline_Left Play)
      (:Update
        (Class|PhysicsConstraintComponent|SetLinearZLimit _physicsconstraintleft "LCM_Limited" (Math|Float|Lerp 0.0 (Variables|Default|GetLimit%20Size) _新建轨道_0))
        (Class|PhysicsConstraintComponent|SetLinearPositionTarget _physicsconstraintleft (Math|Vector|MakeVector 0.0 0.0 (Math|Float|Lerp 0.0 (Variables|Default|GetLimit%20Size) _新建轨道_0)))))
    (else
      (Timeline|timeline_Left Reverse))))

(event Custom|Spawn
  (Input|DisableInput (Game|GetPlayerController 0))
  (Utilities|FlowControl|Delay 0.5)
  (Actor|DestroyActor)
  (bind _returnvalue (Game|SpawnActorfromClass "BP_Player_C" (Transformation|GetActorTransform (Utilities|ResolveSoftReference (Variables|Default|GetPlayerStart))) "Undefined" 0 0))
  (Pawn|Possess (Game|GetPlayerController 0) _returnvalue))

(event Custom|Reset
  (Utilities|FlowControl|DoOnce false) ; enters at Reset
)

(event EventBeginPlay
  (bind _returnvalue (Game|GetPlayerController 0))
  (CallFunction|Init)
  (Variables|/Script/Engine.PlayerController|SetbShowMouseCursor _returnvalue true)
  (Input|DisableInput _returnvalue)
  (EventDispatchers|BindEventtoEventSpawn (EventDispatchers|CreateEvent :!event Custom|Spawn))
  (Utilities|FlowControl|Delay 1.0)
  (Input|EnableInput _returnvalue)
  (CallFunction|UP -1e+01)
  (if (Variables|Default|GetisPC)
    (Variables|Default|SetStepValue (Math|Float|Absolute(Float) (Variables|Default|GetStepValue)))))

(event EventTick
  (params (DeltaSeconds :type Float%20%28single-precision%29))
  (bind _sceneleft (Variables|Default|GetSceneLeft))
  (bind _sceneright (Variables|Default|GetSceneRight))
  (bind _returnvalue (Transformation|GetWorldLocation _sceneleft))
  (bind _returnvalue_2 (Transformation|GetWorldLocation _sceneright))
  (Collision|LineTraceByChannel (Transformation|GetWorldLocation (Variables|Default|GetSceneBody)) (Math|Vector|MakeVector (/ (+ (.x _returnvalue) (.x _returnvalue_2)) 2.0) (/ (+ (.y _returnvalue) (.y _returnvalue_2)) 2.0) (Math|Float|Min(Float) (.z _returnvalue) (.z _returnvalue_2))) "TraceTypeQuery1" false 0 "ForDuration"))

(event Input|AxisEvents|InputAxisMoveLeft
  (params (AxisValue :type Float%20%28single-precision%29))
  (if (Variables|Default|GetisPressLeft)
    (CallFunction|StepLeg AxisValue true)))

(event Input|AxisEvents|InputAxisMoveRight
  (params (AxisValue :type Float%20%28single-precision%29))
  (if (Variables|Default|GetisPressRight)
    (CallFunction|StepLeg AxisValue false)))

(event Input|AxisEvents|InputAxisUP
  (params (AxisValue :type Float%20%28single-precision%29))
  (CallFunction|UP AxisValue))

(event Input|AxisEvents|InputAxisMove
  (params (AxisValue :type Float%20%28single-precision%29))
  (if (not (Variables|Default|GetisPC))
    (if (> (Class|PlayerController|GetInputKeyTimeDown (Game|GetPlayerController 0) "MouseY") 0.0)
      (Utilities|FlowControl|Sequence
        (:then_0
          (Utilities|FlowControl|DoOnce false
            (:Completed
              (switch int (Variables|Default|GetLiftNum)
                (:0
                  (CallFunction|LIftLeft true))
                (:1
                  (CallFunction|LiftRight true))))))
        (:then_1
          (Utilities|FlowControl|Sequence
            (:then_0
              (switch int (Variables|Default|GetLiftNum)
                (:0
                  (Variables|Default|SetLiftNum 0)
                  (CallFunction|StepLeg AxisValue true))
                (:1
                  (Variables|Default|SetLiftNum 1)
                  (CallFunction|StepLeg AxisValue false))))
            (:then_1
              (goto _label Reset)))))
      (else
        (Utilities|FlowControl|DoOnce true :!label _label
          (:Completed
            (Utilities|FlowControl|Sequence
              (:then_0
                (CallFunction|IsCanChange))
              (:then_1
                (CallFunction|Reset)))))))))

(event Input|MouseEvents|RightMouseButton
  (params (Key :type Key%20Structure :default "None"))
  (:Pressed
    (if (Variables|Default|GetisPC)
      (CallFunction|LiftRight true)
      (Variables|Default|SetisPressRight true)))
  (:Released
    (CallFunction|LiftRight false)
    (Variables|Default|SetisPressRight false)))

(event Input|MouseEvents|LeftMouseButton
  (params (Key :type Key%20Structure :default "None"))
  (:Pressed
    (CallFunction|LIftLeft true)
    (Variables|Default|SetisPressLeft true))
  (:Released
    (CallFunction|LIftLeft false)
    (Variables|Default|SetisPressLeft false)))

(fn ConstructionScript)

(fn StepLeg
  (params (value :type Float%20%28single-precision%29) (isLeft :type Boolean))
  (LocalVariables|Set_isLeft isLeft)
  (Physics|AddImpulseatLocation (select (LocalVariables|Get_isLeft) (Variables|Default|GetLeft) (Variables|Default|GetRight)) (* (Math|Vector|GetForwardVector (select (LocalVariables|Get_isLeft) (Variables|Default|GetLeft) (Variables|Default|GetRight))) (* (* value (Math|Float|SelectFloat 1.0 1e+01 (Variables|Default|GetisPC))) (Variables|Default|GetStepValue))) (Transformation|GetWorldLocation (select (LocalVariables|Get_isLeft) (Variables|Default|GetSceneLeft) (Variables|Default|GetSceneRight))) "None"))

(fn UP
  (params (value :type Float%20%28single-precision%29))
  (Physics|AddImpulse (Variables|Default|GetBody) (* (Math|Vector|GetForwardVector (Transformation|GetWorldRotation (Variables|Default|GetBody))) (* value (Variables|Default|Getmove))) "None" false))

(fn IsCanChange
  (bind _scenebody (Variables|Default|GetSceneBody))
  (bind _sceneleft (Variables|Default|GetSceneLeft))
  (bind _sceneright (Variables|Default|GetSceneRight))
  (bind _returnvalue (Transformation|GetWorldLocation _scenebody))
  (bind _returnvalue_2 (Transformation|GetWorldLocation _sceneleft))
  (bind _returnvalue_3 (Transformation|GetWorldLocation _sceneright))
  (bind _returnvalue_4 (+ (.y _returnvalue_2) (.y _returnvalue_3)))
  (bind _returnvalue_5 (+ (.x _returnvalue_2) (.x _returnvalue_3)))
  (bind _returnvalue_6 (Math|Float|Min(Float) (.z _returnvalue_2) (.z _returnvalue_3)))
  (bind _returnvalue_7 (/ _returnvalue_5 2.0))
  (bind _returnvalue_8 (/ _returnvalue_4 2.0))
  (bind _returnvalue_9 (Math|Vector|MakeVector _returnvalue_7 _returnvalue_8 _returnvalue_6))
  (bind _returnvalue_10 (Math|Vector|GetUnitDirection(Vector) _returnvalue_9 _returnvalue))
  (switch int (Variables|Default|GetLiftNum)
    (:0
      (CallFunction|LIftLeft false)
      (if (>= (* (Class|KismetMathLibrary|DegAcos (Math|Vector|DotProduct _returnvalue_10 (Math|Vector|GetUpVector (Utilities|Select :Index (Variables|Default|GetLiftNum) :Option%200 (Variables|Default|GetLeft) :Option%201 (Variables|Default|GetRight))))) (Math|Float|Sign(Float) (Class|KismetMathLibrary|VectorCosineAngle2D (Math|Vector|CrossProduct _returnvalue_10 (Math|Vector|GetUpVector (Utilities|Select :Index (Variables|Default|GetLiftNum) :Option%200 (Variables|Default|GetLeft) :Option%201 (Variables|Default|GetRight)))) "-1.000000,-1.000000,1.000000"))) 0.0)
        (Variables|Default|SetLiftNum 1)
        (Development|PrintString "换成右腿" true true "(R=1.000000,G=0.000000,B=0.217311,A=1.000000)" 3.0)))
    (:1
      (CallFunction|LiftRight false)
      (if (>= (* (Class|KismetMathLibrary|DegAcos (Math|Vector|DotProduct _returnvalue_10 (Math|Vector|GetUpVector (Utilities|Select :Index (Variables|Default|GetLiftNum) :Option%200 (Variables|Default|GetLeft) :Option%201 (Variables|Default|GetRight))))) (Math|Float|Sign(Float) (Class|KismetMathLibrary|VectorCosineAngle2D (Math|Vector|CrossProduct _returnvalue_10 (Math|Vector|GetUpVector (Utilities|Select :Index (Variables|Default|GetLiftNum) :Option%200 (Variables|Default|GetLeft) :Option%201 (Variables|Default|GetRight)))) "-1.000000,-1.000000,1.000000"))) 0.0)
        (Variables|Default|SetLiftNum 0)
        (Development|PrintString "换成左腿" true true "(R=0.000000,G=0.774723,B=1.000000,A=1.000000)" 3.0)))))

(fn Init
  (bind _returnvalue (Rendering|Material|CreateDynamicMaterialInstance (Variables|Default|GetLeft) 0 0 "None" :!class /Script/Engine.PrimitiveComponent))
  (Variables|Default|Set%20LeftMaterialInstance _returnvalue)
  (bind _returnvalue_2 (Rendering|Material|CreateDynamicMaterialInstance (Variables|Default|GetRight) 0 0 "None" :!class /Script/Engine.PrimitiveComponent))
  (Variables|Default|SetRightMaterialInstance _returnvalue_2)
  (Class|PhysicsConstraintComponent|SetAngularSwing2Limit (Variables|Default|GetPhysicsConstraintLeft) "ACM_Limited" (Variables|Default|GetSwing%202Limit%20Angle)))