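; BP_Leg is a physics-driven leg actor that expects a BP_Pawn as its parent actor.
; LiftLeg pushes the Cylinder along the actor's up vector, while StepLeg and Up apply scaled forward impulses at two separate scene-component locations.
; On BeginPlay it makes StepValue positive when the parent pawn's IsPC flag is set.
; A test event prints and raises the cylinder's height above the actor.
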(event Custom|Up
  (params (A :type Float%20%28single-precision%29))
  (Physics|AddImpulseatLocation (Variables|Default|GetCylinder) (* (Transformation|GetActorForwardVector) (* A (Variables|Default|Getmove))) (Transformation|GetWorldLocation (Variables|Default|GetScene1)) "None"))

(event Custom|StepLeg
  (params (Value :type Float%20%28single-precision%29))
  (Physics|AddImpulseatLocation (Variables|Default|GetCylinder) (* (Transformation|GetActorForwardVector) (* Value (Variables|Default|GetStepValue))) (Transformation|GetWorldLocation (Variables|Default|GetScene)) "None"))

(event Custom|test
  (bind _returnvalue (Transformation|GetActorLocation))
  (bind _returnvalue_2 (+ (.z _returnvalue) 3e+02))
  (Development|PrintString (Utilities|String|ToString(Float) _returnvalue_2))
  (Transformation|SetWorldLocation (Variables|Default|GetCylinder) (Math|Vector|MakeVector (.x _returnvalue) (.y _returnvalue) _returnvalue_2) false false))

(event Custom|LiftLeg
  (params (value :type Float%20%28single-precision%29))
  (Physics|AddImpulse (Variables|Default|GetCylinder) (* (Transformation|GetActorUpVector) (* value 4e+02)) "None" false))

(event EventBeginPlay
  (bind _asbp_pawn (Utilities|Casting|CastToBP_Pawn (Actor|GetParentActor)))
  (bind _output_get (Variables|Default|SetAs%20BP%20Pawn _asbp_pawn))
  (if (Variables|/Game/Blueprints/BP_Pawn.BP_Pawn_C|GetisPC _output_get)
    (Variables|Default|SetStepValue (Math|Float|Absolute(Float) (Variables|Default|GetStepValue)))))

(fn ConstructionScript)