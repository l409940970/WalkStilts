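; Physics-driven two-legged player pawn that walks by lifting a leg and pushing with impulses.
; Right mouse lifts the right leg through timeline-driven constraint linear drives, while MoveRight impulses the left leg; left-side input is disconnected.
; Tick pushes the body forward, straightens it when the feet-to-body vector nears vertical, and places leg meat meshes via bone traces.
; BeginGame blends the camera over, then possesses the pawn.
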(event OnComponentBeginOverlap(Sphere)
  (params (OverlappedComponent :type Primitive%20Component%20Object%20Reference) (OtherActor :type Actor%20Object%20Reference) (OtherComp :type Primitive%20Component%20Object%20Reference) (OtherBodyIndex :type Integer) (bFromSweep :type Boolean) (SweepResult :type Hit%20Result%20Structure%20%28by%20ref%29))
  (Collision|SetCollisionEnabled (Variables|Default|GetSphere) "PhysicsOnly"))

(event Custom|LiftRight
  (params (isLift :type Boolean))
  (bind _physicsconstraintright (Variables|Default|GetPhysicsConstraintRight))
  (Variables|Default|SetisLiftRight isLift)
  (CallFunction|ChangeAnim isLift)
  (if isLift
    (bind _新建轨道_0 (Timeline|timeline_Right Play)
      (:Update
        (Class|PhysicsConstraintComponent|SetLinearDriveParams _physicsconstraintright (Math|Float|Lerp 0.0 (Variables|Default|GetPositionStrength) _新建轨道_0) 0.0 0.0)
        (Class|PhysicsConstraintComponent|SetLinearZLimit _physicsconstraintright "LCM_Limited" (Math|Float|Absolute(Float) (Math|Float|Lerp 0.0 (Variables|Default|GetLimitSize) _新建轨道_0)))
        (Class|PhysicsConstraintComponent|SetLinearPositionTarget _physicsconstraintright (Math|Vector|MakeVector 0.0 0.0 (Math|Float|Lerp 0.0 (Variables|Default|GetLimitSize) _新建轨道_0)))))
    (else
      (Rendering|Material|SetVectorParameterValue (Variables|Default|GetRightMaterialInstance) "Color" "(R=1.000000,G=1.000000,B=1.000000,A=1.000000)" :!class /Script/Engine.MaterialInstanceDynamic)
      (Timeline|timeline_Right Reverse))))

(event Custom|LIftLeft
  (params (isLift :type Boolean))
  (bind _physicsconstraintleft (Variables|Default|GetPhysicsConstraintLeft))
  (Variables|Default|SetisLiftLeft isLift)
  (CallFunction|ChangeAnim isLift)
  (if isLift
    (bind _新建轨道_0 (Timeline|timeline_Left Play)
      (:Update
        (Utilities|FlowControl|Sequence
          (:then_0
            (Class|PhysicsConstraintComponent|SetLinearDriveParams _physicsconstraintleft (Math|Float|Lerp 0.0 (Variables|Default|GetPositionStrength) _新建轨道_0) 0.0 0.0)
            (Class|PhysicsConstraintComponent|SetLinearZLimit _physicsconstraintleft "LCM_Limited" (Math|Float|Absolute(Float) (Math|Float|Lerp 0.0 (Variables|Default|GetLimitSize) _新建轨道_0)))
            (Class|PhysicsConstraintComponent|SetLinearPositionTarget _physicsconstraintleft (Math|Vector|MakeVector 0.0 0.0 (Math|Float|Lerp 0.0 (Variables|Default|GetLimitSize) _新建轨道_0)))))))
    (else
      (Rendering|Material|SetVectorParameterValue (Variables|Default|Get%20LeftMaterialInstance) "Color" "(R=1.000000,G=1.000000,B=1.000000,A=1.000000)" :!class /Script/Engine.MaterialInstanceDynamic)
      (Timeline|timeline_Left Reverse))))

(event Custom|Line
  (Utilities|FlowControl|Sequence
    (:then_0
      (CallFunction|ChangeMeat (Variables|Default|GetLLeg_Sk) (Variables|Default|GetMeatValue) (Variables|Default|GetLeftMeat) (Variables|Default|GetPhysicsConstraintLeft)))
    (:then_1
      (CallFunction|ChangeMeat (Variables|Default|GetRLeg_SK) (Variables|Default|GetMeatValue) (Variables|Default|GetRightMeat) (Variables|Default|GetPhysicsConstraintRight)))))

(event Custom|Spawn)

(event Custom|BeginGame
  (bind _returnvalue (Game|GetPlayerController 0))
  (bind _self self)
  (Game|Player|SetViewTargetwithBlend _returnvalue _self 0.5 "VTBlend_Linear" 0.0 false)
  (Utilities|FlowControl|Delay 0.5)
  (Pawn|Possess _returnvalue _self)
  (bind _returnvalue_2 (Actor|GetActorOfClass 0))
  (Actor|DestroyActor _returnvalue_2))

(event Custom|Recover
  (CallFunction|UP (Variables|Default|GetinitForceValue))
  (bind _returnvalue (CallFunction|ReturnCenter))
  (Transformation|SetWorldRotation (Variables|Default|GetBody1) "0, 0, 0" false false)
  (if (<= (Class|KismetMathLibrary|DegAcos (Math|Vector|DotProduct _returnvalue "0, 0,1.000000")) 1e+01)
    (if (and (Variables|Default|GetisRecover) (not (Audio|Components|Audio|IsPlaying (Variables|Default|GetTimeline_SetRot))))
      (Variables|Default|SetisRecover false)
      (Variables|Default|SetinitRot (Transformation|GetWorldRotation (Variables|Default|GetBody)))
      (bind _新建轨道_0 (Timeline|Timeline_SetRot PlayFromStart)
        (:Update
          (Transformation|SetWorldRotation (Variables|Default|GetBody) (Math|Rotator|Lerp(Rotator) (Variables|Default|GetinitRot) "0, 0, 0" _新建轨道_0) false false))))
    (else
      (Variables|Default|SetisRecover true))))

(event Custom|OnDead
  (Collision|SetCollisionEnabled (Variables|Default|GetSphere) "PhysicsOnly"))

(event Custom|Reset
  (Utilities|FlowControl|DoOnce false) ; enters at Reset
)

(event EventBeginPlay
  (CallFunction|Init))

(event EventTick
  (params (DeltaSeconds :type Float%20%28single-precision%29))
  (CallFunction|Line)
  (CallFunction|Recover))

(event EventPossessed
  (params (NewController :type Controller%20Object%20Reference))
  (Class|PrimitiveComponent|SetLinearDamping (Variables|Default|GetBody) (Variables|Default|GetBodyLinearDamp))
  (CallFunction|UP (Variables|Default|GetinitForceValue)))

(event EventDestroyed)

(event Input|AxisEvents|InputAxisMoveLeft
  (params (AxisValue :type Float%20%28single-precision%29)))

(event Input|AxisEvents|InputAxisMoveRight
  (params (AxisValue :type Float%20%28single-precision%29))
  (if (Variables|Default|GetisPressRight)
    (CallFunction|Step AxisValue true)))

(event Input|AxisEvents|InputAxisUP
  (params (AxisValue :type Float%20%28single-precision%29))
  (Utilities|FlowControl|Sequence
    (:then_1
      (CallFunction|UP (* AxisValue (* (Utilities|Time|GetWorldDeltaSeconds) 1.2e+02))))))

(event Input|AxisEvents|InputAxisMove
  (params (AxisValue :type Float%20%28single-precision%29)))

(event Input|MouseEvents|RightMouseButton
  (params (Key :type Key%20Structure))
  (:Pressed
    (CallFunction|LiftRight true)
    (Variables|Default|SetisPressRight true))
  (:Released
    (CallFunction|LiftRight false)
    (Variables|Default|SetisPressRight false)))

(event Input|MouseEvents|LeftMouseButton
  (params (Key :type Key%20Structure)))

(fn ConstructionScript)

(fn BPStep
  (params (value :type Float%20%28single-precision%29) (isLeft :type Boolean))
  (LocalVariables|Set_isLeft isLeft)
  (Physics|AddImpulseatLocation (select (LocalVariables|Get_isLeft) (Variables|Default|GetLeftLeg) (Variables|Default|GetRightLeg)) (* (Math|Vector|GetForwardVector (select (LocalVariables|Get_isLeft) (Variables|Default|GetLeftLeg) (Variables|Default|GetRightLeg))) (* value (Variables|Default|GetStepValue))) (Transformation|GetWorldLocation (select (LocalVariables|Get_isLeft) (Variables|Default|GetSceneLeft) (Variables|Default|GetSceneRight))) "None"))

(fn BPUP
  (params (value :type Float%20%28single-precision%29))
  (Physics|AddImpulse (Variables|Default|GetBody) (* (* (Math|Vector|GetForwardVector (Variables|Default|GetBody)) value) (Variables|Default|GetMove)) "None" false))

(fn BPInit
  (Utilities|FlowControl|Sequence
    (:then_1
      (Class|PhysicsConstraintComponent|SetAngularSwing2Limit (Variables|Default|GetPhysicsConstraintLeft) "ACM_Limited" (Variables|Default|GetSwing%202Limit%20Angle)))))

(fn BPReturnAngle
  (bind _leftleg (Variables|Default|GetLeftLeg))
  (bind _rightleg (Variables|Default|GetRightLeg))
  (bind _liftnum (Variables|Default|GetLiftNum))
  (bind _returnvalue (Utilities|Select :Index _liftnum :Option%200 _leftleg :Option%201 _rightleg))
  (bind _returnvalue_2 (Math|Vector|GetUpVector _returnvalue))
  (bind _returnvalue_3 (CallFunction|ReturnCenter))
  (return (* (Class|KismetMathLibrary|DegAcos (Math|Vector|DotProduct _returnvalue_3 _returnvalue_2)) (Math|Float|Sign(Float) (Class|KismetMathLibrary|VectorCosineAngle2D (Math|Vector|CrossProduct _returnvalue_3 _returnvalue_2) "-1.000000,-1.000000,1.000000")))))

(fn BPReturnCenter
  (bind _sceneleft (Variables|Default|GetSceneLeft))
  (bind _sceneright (Variables|Default|GetSceneRight))
  (bind _returnvalue (Transformation|GetWorldLocation _sceneleft))
  (bind _returnvalue_2 (Transformation|GetWorldLocation _sceneright))
  (return (Math|Vector|GetUnitDirection(Vector) (Math|Vector|MakeVector (/ (+ (.x _returnvalue) (.x _returnvalue_2)) 2.0) (/ (+ (.y _returnvalue) (.y _returnvalue_2)) 2.0) (Math|Float|Min(Float) (.z _returnvalue) (.z _returnvalue_2))) (Transformation|GetWorldLocation (Variables|Default|GetSceneBody)))))

(fn BPLeftLeg
  (switch int (Variables|Default|GetLiftNum)
    (:0
      (CallFunction|LIftLeft true))
    (:1
      (CallFunction|LiftRight true))))

(fn BPStepLeg
  (params (value :type Float%20%28single-precision%29))
  (switch int (Variables|Default|GetLiftNum)
    (:0
      (Variables|Default|SetLiftNum 0)
      (CallFunction|Step value true))
    (:1
      (Variables|Default|SetLiftNum 1)
      (CallFunction|Step value false))))

(fn BPReturnLegDistance
  (return (Math|Vector|Distance(Vector) (Math|Vector|MakeVector (.x (Transformation|GetWorldLocation (Variables|Default|GetSceneLeft))) 0.0 0.0) (Math|Vector|MakeVector (.x (Transformation|GetWorldLocation (Variables|Default|GetSceneRight))) 0.0 0.0))))

(fn SetSkin)

(fn IsChange
  (params (value :type Float%20%28single-precision%29))
  (return (>= value 0.0)))

(fn ChangeAnim
  (params (isLift :type Boolean))
  (Components|Timeline|SetPlayRate (Variables|Default|GetSkelBody) (select isLift 0.8 0.5)))

(fn ChangeMeat
  (params (Lerg :type Scene%20Component%20Object%20Reference) (value :type Integer) (meat :type Scene%20Component%20Object%20Reference) (physicsconstrain :type Physics%20Constraint%20Component%20Object%20Reference))
  (bind _returnvalue (Transformation|GetSocketLocation Lerg "Bone008"))
  (bind _returnvalue_2 (Transformation|GetSocketLocation Lerg "Bone007"))
  (bind _outhit (Collision|LineTraceByChannel _returnvalue _returnvalue_2 "TraceTypeQuery3" false 0 "None" false))
  (Transformation|SetWorldLocation meat (+ (.Location (Collision|BreakHitResult _outhit)) (* (Math|Vector|Normalize (- _returnvalue_2 _returnvalue)) value)) false false)
  (Transformation|SetRelativeRotation meat (Math|Rotator|MakeRotator 16.0 (Class|PhysicsConstraintComponent|GetCurrentSwing2 physicsconstrain) 0.0) false false))