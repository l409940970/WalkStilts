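; Player pawn for physics-based walking, built from a BP_Body child actor and two BP_Leg child actors.
; Timelines lift each leg by driving its physics constraint's Z limit and position target.
; On PC, held mouse buttons lift legs and axis input steps them; otherwise, MoveAll input steps alternating legs, switching between drags.
; A bound spawn event destroys the pawn, then spawns and possesses a replacement at PlayerStart.
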(event Custom|LiftRight
  (params (isLift :type Boolean))
  (bind _physicsconstraintright (Variables|Default|GetPhysicsConstraintRight))
  (if isLift
    (bind _新建轨道_0 (Timeline|timeline_Right Play)
      (:Update
        (Class|PhysicsConstraintComponent|SetLinearZLimit _physicsconstraintright "LCM_Limited" (Math|Float|Lerp 0.0 (Variables|Default|GetLimit%20Size) _新建轨道_0))
        (Class|PhysicsConstraintComponent|SetLinearPositionTarget _physicsconstraintright (Math|Vector|MakeVector 0.0 0.0 (Math|Float|Lerp 0.0 (Variables|Default|GetLimit%20Size) _新建轨道_0)))))
    (else
      (Timeline|timeline_Right Reverse))))

(event Custom|LIftLeft
  (params (isLift :type Boolean))
  (bind _physicsconstraintleft (Variables|Default|GetPhysicsConstraintLeft))
  (if isLift
    (bind _新建轨道_0 (Timeline|timeline_Left Play)
      (:Update
        (Class|PhysicsConstraintComponent|SetLinearZLimit _physicsconstraintleft "LCM_Limited" (Math|Float|Lerp 0.0 (Variables|Default|GetLimit%20Size) _新建轨道_0))
        (Class|PhysicsConstraintComponent|SetLinearPositionTarget _physicsconstraintleft (Math|Vector|MakeVector 0.0 0.0 (Math|Float|Lerp 0.0 (Variables|Default|GetLimit%20Size) _新建轨道_0)))))
    (else
      (Timeline|timeline_Left Reverse))))

(event Custom|Spawn
  (Input|DisableInput (Game|GetPlayerController 0))
  (Utilities|FlowControl|Delay 0.5)
  (Actor|DestroyActor)
  (bind _returnvalue (Game|SpawnActorfromClass "BP_Pawn_C" (Transformation|GetActorTransform (Utilities|ResolveSoftReference (Variables|Default|GetPlayerStart))) "Undefined" 0 0))
  (Pawn|Possess (Game|GetPlayerController 0) _returnvalue))

(event Custom|Reset
  (Utilities|FlowControl|DoOnce false) ; enters at Reset
)

(event EventBeginPlay
  (bind _returnvalue (Game|GetPlayerController 0))
  (Variables|/Script/Engine.PlayerController|SetbShowMouseCursor _returnvalue (not (Variables|Default|GetisPC)))
  (Input|DisableInput _returnvalue)
  (EventDispatchers|BindEventtoEventSpawn (EventDispatchers|CreateEvent :!event Custom|Spawn))
  (CallFunction|InitValue)
  (Utilities|FlowControl|Delay 0.5)
  (Input|EnableInput _returnvalue))

(event Input|AxisEvents|InputAxisMoveAll
  (params (AxisValue :type Float%20%28single-precision%29))
  (if (not (Variables|Default|GetisPC))
    (if (> (Class|PlayerController|GetInputKeyTimeDown (Game|GetPlayerController 0) "MouseY") 0.0)
      (Utilities|FlowControl|Sequence
        (:then_0
          (Utilities|FlowControl|DoOnce false
            (:Completed
              (switch int (Variables|Default|GetLiftNum)
                (:0
                  (CallFunction|LIftLeft true))
                (:1
                  (CallFunction|LiftRight true))))))
        (:then_1
          (Utilities|FlowControl|Sequence
            (:then_0
              (switch int (Variables|Default|GetLiftNum)
                (:0
                  (Variables|Default|SetLiftNum 0)
                  (Default|StepLeg (Variables|Default|GetLeftActor) AxisValue))
                (:1
                  (Variables|Default|SetLiftNum 1)
                  (Default|StepLeg (Variables|Default|GetrightActor) AxisValue))))
            (:then_1
              (goto _label Reset)))))
      (else
        (Utilities|FlowControl|DoOnce true :!label _label
          (:Completed
            (Utilities|FlowControl|Sequence
              (:then_0
                (switch int (Variables|Default|GetLiftNum)
                  (:0
                    (CallFunction|LIftLeft false)
                    (Variables|Default|SetLiftNum 1)
                    (Development|PrintString "换成右腿" true true "(R=1.000000,G=0.000000,B=0.217311,A=1.000000)" 3.0))
                  (:1
                    (CallFunction|LiftRight false)
                    (Variables|Default|SetLiftNum 0)
                    (Development|PrintString "换成左腿" true true "(R=0.000000,G=0.774723,B=1.000000,A=1.000000)" 3.0))))
              (:then_1
                (CallFunction|Reset)))))))))

(event Input|AxisEvents|InputAxisPressLeft
  (params (AxisValue :type Float%20%28single-precision%29)))

(event Input|AxisEvents|InputAxisPressRight
  (params (AxisValue :type Float%20%28single-precision%29)))

(event Input|AxisEvents|InputAxisUP
  (params (AxisValue :type Float%20%28single-precision%29))
  (Default|Up (Variables|Default|GetBodyActor) AxisValue))

(event Input|AxisEvents|InputAxisMoveLif
  (params (AxisValue :type Float%20%28single-precision%29))
  (if (Variables|Default|GetisPressLeft)
    (Default|StepLeg (Variables|Default|GetLeftActor) AxisValue)))

(event Input|AxisEvents|InputAxisMoveRig
  (params (AxisValue :type Float%20%28single-precision%29))
  (if (Variables|Default|GetisPressRight)
    (Default|StepLeg (Variables|Default|GetrightActor) AxisValue)))

(event Input|MouseEvents|RightMouseButton
  (params (Key :type Key%20Structure))
  (:Pressed
    (if (Variables|Default|GetisPC)
      (CallFunction|LiftRight true)
      (Variables|Default|SetisPressRight true)))
  (:Released
    (CallFunction|LiftRight false)
    (Variables|Default|SetisPressRight false)))

(event Input|MouseEvents|LeftMouseButton
  (params (Key :type Key%20Structure))
  (:Pressed
    (CallFunction|LIftLeft true)
    (Variables|Default|SetisPressLeft true))
  (:Released
    (CallFunction|LIftLeft false)
    (Variables|Default|SetisPressLeft false)))

(fn ConstructionScript)

(fn InitValue
  (bind _asbp_body (Utilities|Casting|CastToBP_Body (Variables|/Script/Engine.ChildActorComponent|GetChildActor (Variables|Default|GetBody))))
  (Variables|Default|SetBodyActor _asbp_body)
  (bind _asbp_leg (Utilities|Casting|CastToBP_Leg (Variables|/Script/Engine.ChildActorComponent|GetChildActor (Variables|Default|GetRight))))
  (Variables|Default|SetrightActor _asbp_leg)
  (bind _asbp_leg_2 (Utilities|Casting|CastToBP_Leg (Variables|/Script/Engine.ChildActorComponent|GetChildActor (Variables|Default|GetLeft))))
  (Variables|Default|SetLeftActor _asbp_leg_2)
  (Class|PhysicsConstraintComponent|SetAngularSwing2Limit (Variables|Default|GetPhysicsConstraintLeft) "ACM_Limited" (Variables|Default|GetSwing%202Limit%20Angle)))

(fn 1111
  (params (NewParam :type Boolean))
  (if NewParam
    (Development|PrintString "Hello")
    (else
      (Development|PrintString "no"))))