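; BP_Pawn1 is a physics-driven walker pawn built from a body and two leg child actors, cached on BeginPlay.
; Up input drives the body, while mouse buttons retarget physics constraints, with right click raising and releasing the right side's Z target.
; Holding right mouse lets MoveRig step the right leg.
; The left leg's matching Move step is gated by a flag that only disconnected nodes set.
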(event EventBeginPlay
  (bind _asbp_body (Utilities|Casting|CastToBP_Body (Variables|/Script/Engine.ChildActorComponent|GetChildActor (Variables|Default|GetBody))))
  (Variables|Default|SetBodyActor _asbp_body)
  (bind _asbp_leg (Utilities|Casting|CastToBP_Leg (Variables|/Script/Engine.ChildActorComponent|GetChildActor (Variables|Default|GetRight))))
  (Variables|Default|SetrightActor _asbp_leg)
  (bind _asbp_leg_2 (Utilities|Casting|CastToBP_Leg (Variables|/Script/Engine.ChildActorComponent|GetChildActor (Variables|Default|GetLeft))))
  (Variables|Default|SetLeftActor _asbp_leg_2))

(event Input|AxisEvents|InputAxisMove
  (params (AxisValue :type Float%20%28single-precision%29))
  (if (Variables|Default|GetisPressLeft)
    (Default|StepLeg (Variables|Default|GetLeftActor) AxisValue)))

(event Input|AxisEvents|InputAxisUP
  (params (AxisValue :type Float%20%28single-precision%29))
  (Default|Up (Variables|Default|GetBodyActor) AxisValue))

(event Input|AxisEvents|InputAxisMoveRig
  (params (AxisValue :type Float%20%28single-precision%29))
  (if (Variables|Default|GetisPressRight)
    (Default|StepLeg (Variables|Default|GetrightActor) AxisValue)))

(event Input|MouseEvents|RightMouseButton
  (params (Key :type Key%20Structure))
  (bind _physicsconstraintright (Variables|Default|GetPhysicsConstraintRight))
  (bind _physicsconstraintright_2 (Variables|Default|GetPhysicsConstraintRight))
  (:Pressed
    (Class|PhysicsConstraintComponent|SetLinearZLimit _physicsconstraintright "LCM_Limited" 5e+02)
    (Class|PhysicsConstraintComponent|SetLinearPositionTarget _physicsconstraintright (Math|Vector|MakeVector 0.0 0.0 5e+02))
    (Class|PhysicsConstraintComponent|SetAngularSwing2Limit _physicsconstraintright "ACM_Limited" 45.0)
    (Variables|Default|SetisPressRight true))
  (:Released
    (Class|PhysicsConstraintComponent|SetLinearZLimit _physicsconstraintright_2 "LCM_Limited" 5e+02)
    (Class|PhysicsConstraintComponent|SetLinearPositionTarget _physicsconstraintright_2 (Math|Vector|MakeVector 0.0 0.0 0.0))
    (Variables|Default|SetisPressRight false)))

(event Input|MouseEvents|LeftMouseButton
  (params (Key :type Key%20Structure))
  (bind _physicsconstraintleft1 (Variables|Default|GetPhysicsConstraintleft1))
  (:Pressed
    (Class|PhysicsConstraintComponent|SetAngularTwistLimit _physicsconstraintleft1 "ACM_Limited" 3e+01)
    (Class|PhysicsConstraintComponent|SetAngularOrientationTarget _physicsconstraintleft1 (Math|Rotator|MakeRotator 0.0 0.0 3e+01))))

(fn ConstructionScript)