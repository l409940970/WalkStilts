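; Level game mode that hides the mouse cursor and handles player spawning and respawning.
; On begin play it binds a restart-game event, then spawns BP_Player_main at the PlayerStart it finds and moves any current player pawn there, without possessing the spawned one.
; A restart destroys the current pawn, runs the same spawn function and has the player controller possess the new pawn.
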(event Custom|BaseInit
  (EventDispatchers|BindEventtoEventRestartGame (delegate Custom|SpawnNewPlayer)))

(event Custom|SpawnNewPlayer
  (Actor|DestroyActor (Game|Player|GetPlayerPawn 0))
  (bind _returnvalue (CallFunction|SpwanPlayer))
  (Utilities|IsValid _returnvalue
    (:Is%20Valid
      (Pawn|Possess (Game|GetPlayerController 0) _returnvalue))))

(event EventBeginPlay
  (Variables|/Script/Engine.PlayerController|SetbShowMouseCursor (Game|GetPlayerController 0) false)
  (CallFunction|BaseInit)
  (CallFunction|SpwanPlayer))

(fn ConstructionScript
  (|CallParentFunction))

(fn SpwanPlayer
  (bind _returnvalue (Game|Player|GetPlayerPawn 0))
  (bind _returnvalue_2 (Actor|GetActorOfClass "/Script/Engine.PlayerStart"))
  (Utilities|IsValid _returnvalue_2
    (:Is%20Valid
      (Variables|Default|SetstartLocation (Math|Vector|MakeVector (.x (.location (Transformation|GetActorTransform _returnvalue_2))) (.y (.location (Transformation|GetActorTransform _returnvalue_2))) (.z (.location (Transformation|GetActorTransform _returnvalue_2)))))
      (bind _returnvalue_3 (Game|SpawnActorfromClass "/Game/GamePlay/Blueprints/Player/BP_Player_main.BP_Player_main_C" (Math|Transform|MakeTransform (Math|Vector|MakeVector (.x (.location (Transformation|GetActorTransform _returnvalue_2))) (.y (.location (Transformation|GetActorTransform _returnvalue_2))) (.z (.location (Transformation|GetActorTransform _returnvalue_2)))) (.rotation (Transformation|GetActorTransform _returnvalue_2)) (.scale (Transformation|GetActorTransform _returnvalue_2))) "Undefined" (Game|GetPlayerController 0) 0))
      (if (Utilities|IsValid _returnvalue)
        (Transformation|SetActorTransform _returnvalue (Math|Transform|MakeTransform (Math|Vector|MakeVector (.x (.location (Transformation|GetActorTransform _returnvalue_2))) (.y (.location (Transformation|GetActorTransform _returnvalue_2))) (.z (.location (Transformation|GetActorTransform _returnvalue_2)))) (.rotation (Transformation|GetActorTransform _returnvalue_2)) (.scale (Transformation|GetActorTransform _returnvalue_2))) true true))
      (return _returnvalue_3))))