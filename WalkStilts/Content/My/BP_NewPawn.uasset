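; BP_NewPawn is a pawn pushed along its forward vector by physics impulses.
; The UP axis input, scaled by the Move variable, drives an impulse on the Base component.
; Left mouse presses alternate the IsLeft flag through a FlipFlop, though nothing here reads it.
; The Move axis event is empty, and a delayed initial impulse using Init is left disconnected.
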(event EventBeginPlay)

(event Input|AxisEvents|InputAxisUP
  (params (AxisValue :type Float%20%28single-precision%29))
  (Physics|AddImpulse (Variables|Default|Getbase) (* (Transformation|GetActorForwardVector) (* AxisValue (Variables|Default|Getmove))) "None" false))

(event Input|AxisEvents|InputAxisMove
  (params (AxisValue :type Float%20%28single-precision%29)))

(event Input|MouseEvents|LeftMouseButton
  (params (Key :type Key%20Structure :default "None"))
  (:Pressed
    (Utilities|FlowControl|FlipFlop
      (:A
        (Variables|Default|SetisLeft true))
      (:B
        (Variables|Default|SetisLeft false)))))

(fn ConstructionScript)