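; BP_Body is a physics body actor that expects a BP_Pawn as its parent actor and moves by impulses on its Base component.
; On BeginPlay it caches that pawn, then after a short delay applies a backward kick along its forward axis.
; The Up event pushes Base along the forward axis, scaled by its input and Move.
; Any overlap on Sphere calls the pawn's CallEventSpawn.
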(event OnComponentBeginOverlap(Sphere)
  (params (OverlappedComponent :type Primitive%20Component%20Object%20Reference) (OtherActor :type Actor%20Object%20Reference) (OtherComp :type Primitive%20Component%20Object%20Reference) (OtherBodyIndex :type Integer) (bFromSweep :type Boolean) (SweepResult :type Hit%20Result%20Structure%20%28by%20ref%29))
  (bind _as_bp_pawn (Variables|Default|GetAs%20BP%20Pawn))
  (Utilities|IsValid _as_bp_pawn
    (:Is%20Valid
      (Default|CallEventSpawn _as_bp_pawn))))

(event Custom|Up
  (params (A :type Float%20%28single-precision%29))
  (Physics|AddImpulse (Variables|Default|Getbase) (* (Transformation|GetActorForwardVector) (* A (Variables|Default|Getmove))) "None" false))

(event EventBeginPlay
  (bind _asbp_pawn (Utilities|Casting|CastToBP_Pawn (Actor|GetParentActor)))
  (Variables|Default|SetAs%20BP%20Pawn _asbp_pawn)
  (Utilities|FlowControl|Delay 1.0)
  (Physics|AddImpulse (Variables|Default|Getbase) (* (Transformation|GetActorForwardVector) -5e+03) "None" false))

(event EventTick
  (params (DeltaSeconds :type Float%20%28single-precision%29)))

(fn ConstructionScript)